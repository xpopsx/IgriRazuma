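; Actor component on VR_Pawn that provides arc-aimed VR teleportation from a motion controller.
; While active, each tick predicts a projectile path from the controller against WorldStatic objects and projects the hit onto the navmesh.
; Valid targets draw the arc through a shared BP_SplineActor, found in the level or spawned on demand.
; EndTeleport clears the arc and teleports the pawn to the last valid point with zero rotation.
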(event EventBeginPlay
  (Variables|Default|SetVRPawn (CallFunction|GetVRPawn)))

(event EventTick
  (params (DeltaSeconds :type Float%20%28single-precision%29))
  (if (Variables|Default|GetbTeleportActive)
    (bind (_bfindpoint _pointlocation _outpathpositions) (CallFunction|TraceTeleport))
    (bind _output_get (Variables|Default|SetbFindTeleportLocation _bfindpoint))
    (bind _output_get_2 (Variables|Default|SetPoint%20Location _pointlocation))
    (if _output_get
      (CallFunction|UpdateArcVisual _outpathpositions _output_get_2)
      (else
        (Default|ClearSpline (Variables|Default|GetArcSplineActor))))))

(fn TraceTeleport
  (bind _currentmotioncontroller (Variables|Default|GetCurrentMotionController))
  (bind (_outhit _outpathpositions _outlasttracedestination _returnvalue) (Class|GameplayStatics|BlueprintPredictProjectilePathbyObjectType (Transformation|GetWorldLocation _currentmotioncontroller) (* (Math|Vector|GetForwardVector _currentmotioncontroller) (Variables|Default|GetArcVelocity)) true 0.0 (Utilities|Array|MakeArray "ObjectTypeQuery1") false (Utilities|Array|MakeArray (Components|GetOwner self)) "None" 0.0 3e+01))
  (return (and _returnvalue (.ReturnValue (AI|Navigation|ProjectPointtoNavigation (Class|NavigationSystemV1|GetNavigationSystem) (.Location (Collision|BreakHitResult _outhit)) 0 0 (Variables|Default|GetNavigationQueryExtent)))) (select (.ReturnValue (AI|Navigation|ProjectPointtoNavigation (Class|NavigationSystemV1|GetNavigationSystem) (.Location (Collision|BreakHitResult _outhit)) 0 0 (Variables|Default|GetNavigationQueryExtent))) (.ProjectedLocation (AI|Navigation|ProjectPointtoNavigation (Class|NavigationSystemV1|GetNavigationSystem) (.Location (Collision|BreakHitResult _outhit)) 0 0 (Variables|Default|GetNavigationQueryExtent))) (.Location (Collision|BreakHitResult _outhit))) _outpathpositions))

(fn StartTeleport
  (params (MotionController :type Motion%20Controller%20Component%20Object%20Reference))
  (Utilities|IsValid MotionController
    (:Is%20Valid
      (Variables|Default|SetbTeleportActive true)
      (Variables|Default|SetCurrentMotionController MotionController))
    (:Is%20Not%20Valid
      (Variables|Default|SetbTeleportActive false))))

(fn EndTeleport
  (params (CurrentMotionController :type Motion%20Controller%20Component%20Object%20Reference))
  (if (== CurrentMotionController (Variables|Default|GetCurrentMotionController))
    (Variables|Default|SetbTeleportActive false)
    (Variables|Default|SetCurrentMotionController 0)
    (Default|ClearSpline (Variables|Default|GetArcSplineActor))
    (if (Variables|Default|GetbFindTeleportLocation)
      (Transformation|Teleport (Variables|Default|GetVRPawn) (Variables|Default|GetPoint%20Location) "0, 0, 0"))))

(fn UpdateArcVisual
  (params (Points :type Array%20of%20Vectors) (EndPoint :type Vector))
  (bind _arcsplineactor (Variables|Default|GetArcSplineActor))
  (CallFunction|FindArcSplineActor)
  (Default|ClearSpline _arcsplineactor)
  (Default|UpdateSpline _arcsplineactor Points EndPoint))

(fn FindArcSplineActor
  (Utilities|IsValid (Variables|Default|GetArcSplineActor)
    (:Is%20Not%20Valid
      (bind _outactors (Actor|GetAllActorsOfClass "/Game/Core/Blueprints/Teleport/BP_SplineActor.BP_SplineActor_C"))
      (if (!= (Utilities|Array|Length _outactors) 0)
        (for _array_element _outactors
          (Variables|Default|SetArcSplineActor _array_element))
        (else
          (bind _returnvalue (Game|SpawnActorfromClass "/Game/Core/Blueprints/Teleport/BP_SplineActor.BP_SplineActor_C" (Math|Transform|MakeTransform "0, 0, 0") "Undefined" 0 0))
          (Variables|Default|SetArcSplineActor _returnvalue))))))

(fn GetVRPawn
  (bind _asvr_pawn (Utilities|Casting|CastToVR_Pawn (Components|GetOwner))
    (:then
      (return _asvr_pawn))
    (:CastFailed
      (return 0))))