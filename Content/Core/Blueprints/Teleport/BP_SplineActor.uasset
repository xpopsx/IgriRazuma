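; Spline actor in the Teleport folder that draws a curved path with a marker cylinder at its end, likely for teleport aiming.
; UpdateSpline builds the spline from supplied points, adds a spline mesh per segment using the spline's tangents, then moves and reveals the cylinder at the end vector.
; ClearSpline destroys those meshes, clears the points and hides the cylinder.
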(event EventBeginPlay)

(event Collision|EventActorBeginOverlap
  (params (OtherActor :type Actor%20Object%20Reference)))

(event EventTick
  (params (DeltaSeconds :type Float%20%28single-precision%29)))

(fn ConstructionScript)

(fn UpdateSpline
  (params (Points :type Array%20of%20Vectors) (EndVector :type Vector))
  (bind _spline (Variables|Default|GetSpline))
  (for _array_element Points
    (Spline|AddSplinePoint (Variables|Default|GetSpline) _array_element "Local" true))
  (for _index (range 0 (- (Spline|GetNumberOfSplinePoints (Variables|Default|GetSpline)) 2))
    (bind _returnvalue (AddComponent|AddSplineMeshComponent false (Math|Transform|MakeTransform "0, 0, 0")))
    (Utilities|Array|Add (Variables|Default|GetSplineMeshes) _returnvalue)
    (SplineMesh|SetStartandEnd _returnvalue (Utilities|Array|Get(acopy) Points _index) (Spline|GetTangentatSplinePoint _spline _index "Local") (Utilities|Array|Get(acopy) Points (+ _index 1)) (Spline|GetTangentatSplinePoint _spline (+ _index 1) "Local") true :!class /Script/Engine.SplineMeshComponent))
  (Transformation|SetWorldLocation (Variables|Default|GetCylinder) EndVector false false)
  (Development|SetHiddeninGame (Variables|Default|GetCylinder) false true))

(fn ClearSpline
  (bind _splinemeshes (Variables|Default|GetSplineMeshes))
  (for _array_element _splinemeshes
    (Components|DestroyComponent _array_element))
  (Utilities|Array|Clear _splinemeshes)
  (Spline|ClearSplinePoints (Variables|Default|GetSpline) true)
  (Development|SetHiddeninGame (Variables|Default|GetCylinder) true true))