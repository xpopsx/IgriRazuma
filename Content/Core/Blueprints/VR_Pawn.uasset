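; VR player pawn with floor-origin tracking that handles teleporting, ladder climbing and simple falling.
; Teleport input starts and ends teleports through BPTeleportComponent for the pressing controller.
; Grabbing over a BP_Ladder stores that controller and start heights, then Tick moves the pawn vertically against the hand's motion.
; A downward trace below the headset drops the pawn a fixed step per tick when ungrounded and not grabbing.
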(event OnComponentBeginOverlap(GrabCollisionLeft)
  (params (OverlappedComponent :type Primitive%20Component%20Object%20Reference) (OtherActor :type Actor%20Object%20Reference) (OtherComp :type Primitive%20Component%20Object%20Reference) (OtherBodyIndex :type Integer) (bFromSweep :type Boolean) (SweepResult :type Hit%20Result%20Structure%20%28by%20ref%29))
  (Utilities|Casting|CastToBP_Ladder OtherActor))

(event OnComponentBeginOverlap(GrabCollisionRight)
  (params (OverlappedComponent :type Primitive%20Component%20Object%20Reference) (OtherActor :type Actor%20Object%20Reference) (OtherComp :type Primitive%20Component%20Object%20Reference) (OtherBodyIndex :type Integer) (bFromSweep :type Boolean) (SweepResult :type Hit%20Result%20Structure%20%28by%20ref%29))
  (Utilities|Casting|CastToBP_Ladder OtherActor))

(event EventBeginPlay
  (Class|HeadMountedDisplayFunctionLibrary|SetTrackingOrigin "Floor"))

(event Collision|EventActorBeginOverlap
  (params (OtherActor :type Actor%20Object%20Reference)))

(event EventTick
  (params (DeltaSeconds :type Float%20%28single-precision%29))
  (bind _returnvalue (Transformation|GetActorLocation))
  (bind _currentgrabcontroller (Variables|Default|GetCurrentGrabController))
  (Utilities|FlowControl|Sequence
    (:then_0
      (Utilities|IsValid _currentgrabcontroller
        (:Is%20Valid
          (Transformation|SetActorLocation (Math|Vector|MakeVector (.x _returnvalue) (.y _returnvalue) (+ (- (Variables|Default|GetStartRelativeLocationZ) (.z (Variables|/Script/Engine.SceneComponent|GetRelativeLocation _currentgrabcontroller))) (Variables|Default|GetStartOriginZ))) false false))))
    (:then_1
      (CallFunction|SimpleFalling))))

(event Input|ActionEvents|InputActionGrabLeft
  (params (Key :type Key%20Structure :default "None"))
  (bind _motioncontrollerleft (Variables|Default|GetMotionControllerLeft))
  ;[1 1 1] Grab
  (:Pressed
    (CallFunction|Grab _motioncontrollerleft (Variables|Default|GetGrabCollisionLeft)))
  (:Released
    (CallFunction|Release _motioncontrollerleft)))

(event Input|ActionEvents|InputActionGrabRight
  (params (Key :type Key%20Structure :default "None"))
  (bind _motioncontrollerright (Variables|Default|GetMotionControllerRight))
  ;[1 1 1] Grab
  (:Pressed
    (CallFunction|Grab _motioncontrollerright (Variables|Default|GetGrabCollisionRight)))
  (:Released
    (CallFunction|Release _motioncontrollerright)))

(event Input|ActionEvents|InputActionTeleportLeft
  (params (Key :type Key%20Structure :default "None"))
  (bind _motioncontrollerleft (Variables|Default|GetMotionControllerLeft))
  ;[1 1 1] Teleport
  (:Pressed
    (CallFunction|ActionTeleport _motioncontrollerleft true))
  (:Released
    (CallFunction|ActionTeleport _motioncontrollerleft false)))

(event Input|ActionEvents|InputActionTeleportRight
  (params (Key :type Key%20Structure :default "None"))
  (bind _motioncontrollerright (Variables|Default|GetMotionControllerRight))
  ;[1 1 1] Teleport
  (:Pressed
    (CallFunction|ActionTeleport _motioncontrollerright true))
  (:Released
    (CallFunction|ActionTeleport _motioncontrollerright false)))

(fn ConstructionScript)

(fn FadeTeleport
  (params (bFade :type Boolean))
  (CameraFades|StartCameraFade :self (Game|GetPlayerCameraManager 0) :FromAlpha (Math|Float|SelectFloat 0.0 1.0 bFade) :ToAlpha (Math|Float|SelectFloat 1.0 0.0 false) :Duration 0.5))

(fn ActionTeleport
  (params (MC :type Motion%20Controller%20Component%20Object%20Reference) (bPressed :type Boolean))
  (bind _bp_teleportcomponent (Variables|Default|GetBP_TeleportComponent))
  (if bPressed
    (Default|StartTeleport _bp_teleportcomponent MC)
    (else
      (Default|EndTeleport _bp_teleportcomponent MC))))

(fn Grab
  (params (CurrentGrabController :type Motion%20Controller%20Component%20Object%20Reference) (Collision :type Primitive%20Component%20Object%20Reference))
  (if (!= (Utilities|Array|Length (Collision|GetOverlappingActors Collision "/Game/Core/Blueprints/BP_Ladder.BP_Ladder_C" :!class /Script/Engine.PrimitiveComponent)) 0)
    (bind _output_get (Variables|Default|SetCurrentGrabController CurrentGrabController))
    (Utilities|IsValid _output_get
      (:Is%20Valid
        (Variables|Default|SetStartRelativeLocationZ (.z (Variables|/Script/Engine.SceneComponent|GetRelativeLocation _output_get)))
        (Variables|Default|SetStartOriginZ (.z (Transformation|GetActorLocation)))))
    (else
      (Variables|Default|SetCurrentGrabController 0))))

(fn SimpleFalling
  (bind _vrroot (Variables|Default|GetVRRoot))
  (bind _camera (Variables|Default|GetCamera))
  (bind _returnvalue (Transformation|GetWorldLocation _camera))
  (bind _returnvalue_2 (Transformation|GetWorldLocation _vrroot))
  (bind _returnvalue_3 (+ (Math|Vector|MakeVector (.x _returnvalue) (.y _returnvalue) (.z _returnvalue_2)) "0, 0,100.000000"))
  (bind _outhit (Collision|LineTraceByChannel _returnvalue_3 (+ _returnvalue_3 (* (Math|Vector|VectorUp) -1e+03)) "TraceTypeQuery1" false (Utilities|Array|MakeArray self) "None"))
  (if (.bBlockingHit (Collision|BreakHitResult _outhit))
    (if (> (Math|Vector|VectorLength (- (.Location (Collision|BreakHitResult _outhit)) _returnvalue_3)) 1e+02)
      (Utilities|IsValid (Variables|Default|GetCurrentGrabController) :!label _label
        (:Is%20Not%20Valid
          (Transformation|AddActorWorldOffset (Math|Vector|MakeVector 0.0 0.0 -9.8)))))
    (else
      (goto _label))))

(fn Release
  (params (CurrentGrabController :type Motion%20Controller%20Component%20Object%20Reference))
  (if (== CurrentGrabController (Variables|Default|GetCurrentGrabController))
    (Variables|Default|SetCurrentGrabController 0)))